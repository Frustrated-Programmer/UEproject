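; Camera actor that becomes the first player's view target and offers tilt, flip and zoom controls around a root pivot.
; Resize derives a peak height from a width and moves the DirectionalLight there; Zoom halves that height and StopZooming restores it.
; RotateMe tilts the root's roll within soft limits either side of level.
; FlipMe steps pitch toward top or bottom, snapping and returning true when close.
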(event EventBeginPlay)

(event Collision|EventActorBeginOverlap
  (params (OtherActor :type Actor%20Object%20Reference)))

(event EventTick
  (params (DeltaSeconds :type Float%20%28single-precision%29)))

(fn ConstructionScript
  (Transformation|SetWorldRotation (Variables|Default|GetDefaultSceneRoot) (Math|Rotator|MakeRotator (Variables|Default|GetCamRotationX) 0.0 0.0) false false)
  (CallFunction|Resize))

(fn Resize
  (params (Width :type Integer))
  (bind _returnvalue (* Width 75.0))
  (Variables|Default|SetPeak _returnvalue)
  (Transformation|SetRelativeLocation (Variables|Default|GetDirectionalLight) (Math|Vector|MakeVector 0.0 0.0 _returnvalue) false false)
  (Game|Player|SetViewTargetwithBlend (Game|GetPlayerController 0) self 0.0 "VTBlend_Linear" 0.0 false))

(fn RotateMe
  (params (Amount :type Float%20%28single-precision%29))
  (bind _returnvalue (* Amount -1.0))
  (if (and (> (Variables|Default|GetCamRotationX) -8e+01) (< _returnvalue 0.0))
    (bind _output_get (Variables|Default|SetCamRotationX (+ (Variables|Default|GetCamRotationX) _returnvalue) :!label _label))
    (Transformation|SetWorldRotation (Variables|Default|GetDefaultSceneRoot) (Math|Rotator|MakeRotator _output_get (Variables|Default|GetCamRotationY) 0.0) false false)
    (elif (and (< (Variables|Default|GetCamRotationX) 8e+01) (> _returnvalue 0.0))
      (goto _label))))

(fn FlipMe
  (params (Amount :type Float%20%28single-precision%29) (ToTop :type Boolean))
  (Variables|Default|SetCamRotationY (+ Amount (Variables|Default|GetCamRotationY)))
  (Transformation|SetWorldRotation (Variables|Default|GetDefaultSceneRoot self) (Math|Rotator|MakeRotator (Variables|Default|GetCamRotationX) (Variables|Default|GetCamRotationY) 0.0) false false)
  (if (and (not ToTop) (Math|Float|NearlyEqual(Float) (Variables|Default|GetCamRotationY) 1.8e+02 1e+01))
    (Transformation|SetWorldRotation (Variables|Default|GetDefaultSceneRoot self) (Math|Rotator|MakeRotator (Variables|Default|GetCamRotationX) 1.8e+02 0.0) false false)
    (Variables|Default|SetCamRotationY 1.8e+02)
    (elif (or (and ToTop (Math|Float|NearlyEqual(Float) (Variables|Default|GetCamRotationY) 0.0 1e+01)) (and ToTop (Math|Float|NearlyEqual(Float) (Variables|Default|GetCamRotationY) 3.6e+02 1e+01)))
      (Transformation|SetWorldRotation (Variables|Default|GetDefaultSceneRoot self) (Math|Rotator|MakeRotator (Variables|Default|GetCamRotationX) 0.0 0.0) false false)
      (Variables|Default|SetCamRotationY 0.0)
      (else
        (return false))))
  (return true))

(fn Zoom
  (Transformation|SetRelativeLocation (Variables|Default|GetDirectionalLight) (Math|Vector|MakeVector 0.0 0.0 (/ (Variables|Default|GetPeak) 2.0)) false false))

(fn StopZooming
  (Transformation|SetRelativeLocation (Variables|Default|GetDirectionalLight) (Math|Vector|MakeVector 0.0 0.0 (Variables|Default|GetPeak)) false false))