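; Character2 is a movable character that travels in fixed, tile-like steps along world X or Y.
; MoveX and MoveY start a step only when idle and a Visibility line trace to the target is clear, storing one hundredth of the offset.
; Tick advances the location by that increment scaled by the game mode's OverallSpeed until Step reaches 100.
; DoneMoving then resets movement state and clears the game mode's Char2Moving flag.
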(event EventTick
  (params (DeltaSeconds :type Float%20%28single-precision%29))
  (bind _returnvalue (Game|GetGameMode))
  (bind _w_character (Variables|Default|GetW_Character))
  (bind _returnvalue_2 (Transformation|GetWorldLocation _w_character))
  (bind _asthe_game_mode (Utilities|Casting|CastToTheGameMode _returnvalue))
  (bind _overallspeed (Variables|/Game/Blueprints/TheGameMode.TheGameMode_C|GetOverallSpeed _asthe_game_mode))
  (if (Variables|Default|GetMoving)
    (Transformation|SetWorldLocation _w_character (Math|Vector|MakeVector (+ (* _overallspeed (Variables|Default|GetX)) (.x _returnvalue_2)) (+ (* _overallspeed (Variables|Default|GetY)) (.y _returnvalue_2)) (.z _returnvalue_2)) false false)
    (bind _output_get (Variables|Default|SetStep (+ _overallspeed (Variables|Default|GetStep))))
    (if (>= _output_get 1e+02)
      (CallFunction|DoneMoving))))

(fn ConstructionScript)

(fn MoveX
  (params (X :type Float%20%28single-precision%29))
  (bind _w_character (Variables|Default|GetW_Character))
  (bind _returnvalue (Transformation|GetWorldLocation _w_character))
  (bind (_x _y _z) (Math|Vector|BreakVector _returnvalue))
  (if (not (Variables|Default|GetMoving))
    (if (!= X 0.0)
      (bind _returnvalue_2 (Collision|LineTraceByChannel _returnvalue (Math|Vector|MakeVector (+ X _x) _y _z) "TraceTypeQuery1" false 0 "None"))
      (if (not _returnvalue_2)
        (Variables|/Game/Blueprints/TheGameMode.TheGameMode_C|SetChar2Moving (.AsThe%20Game%20Mode (Utilities|Casting|CastToTheGameMode (Game|GetGameMode))) false)
        (Variables|Default|SetMoving true)
        (Variables|Default|SetX (/ X 1e+02))))))

(fn MoveY
  (params (Y :type Float%20%28single-precision%29))
  (bind _w_character (Variables|Default|GetW_Character))
  (bind _returnvalue (Transformation|GetWorldLocation _w_character))
  (bind (_x _y _z) (Math|Vector|BreakVector _returnvalue))
  (if (not (Variables|Default|GetMoving))
    (if (!= Y 0.0)
      (bind _returnvalue_2 (Collision|LineTraceByChannel _returnvalue (Math|Vector|MakeVector _x (+ Y _y) _z) "TraceTypeQuery1" false 0 "None"))
      (if (not _returnvalue_2)
        (Variables|/Game/Blueprints/TheGameMode.TheGameMode_C|SetChar2Moving (.AsThe%20Game%20Mode (Utilities|Casting|CastToTheGameMode (Game|GetGameMode))) false)
        (Variables|Default|SetMoving true)
        (Variables|Default|SetY (/ Y 1e+02))))))

(fn DoneMoving
  (bind _asthe_game_mode (Utilities|Casting|CastToTheGameMode (Game|GetGameMode))
    (:then
      (Variables|/Game/Blueprints/TheGameMode.TheGameMode_C|SetChar2Moving _asthe_game_mode false)
      (Variables|Default|SetMoving false)
      (Variables|Default|SetX 0.0)
      (Variables|Default|SetY 0.0)
      (Variables|Default|SetStep 0.0))
    (:CastFailed
      (Development|PrintString "What happened? Char1 couldn't cast to TheGameMode when DoneMoving" true true "(R=1.000000,G=0.046953,B=0.000000,A=1.000000)" 2e+01))))