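; FloorBox is a floor tile actor that colors itself for a checkerboard pattern based on its world position.
; The construction script offsets the mesh location by 1000 in X and Y, then tests whether each axis is an exact multiple of 200.
; Matching results assign the two grid color materials in one order across both slots, and differing results swap them.
; The event graph holds only disabled placeholder events.
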(event EventBeginPlay)

(event Collision|EventActorBeginOverlap
  (params (OtherActor :type Actor%20Object%20Reference)))

(event EventTick
  (params (DeltaSeconds :type Float%20%28single-precision%29)))

(fn ConstructionScript
  (bind _staticmesh (Variables|Default|GetStaticMesh))
  (bind _staticmesh_2 (Variables|Default|GetStaticMesh))
  (bind _returnvalue (Transformation|GetWorldLocation _staticmesh))
  (bind _returnvalue_2 (+ _returnvalue "1000.000000,1000.000000, 0"))
  (bind _returnvalue_3 (Math|Float|%(Float) (.y _returnvalue_2) 2e+02))
  (bind _returnvalue_4 (== _returnvalue_3 0.0))
  (if (== (Math|Float|%(Float) (.x _returnvalue_2) 2e+02) 0.0)
    (if _returnvalue_4
      (Rendering|Material|SetMaterial _staticmesh_2 0 "/Game/Assets/Materials/Grid_Color_1.Grid_Color_1" :!label _label)
      (Rendering|Material|SetMaterial _staticmesh_2 1 "/Game/Assets/Materials/Grid_Color_2.Grid_Color_2")
      (else
        (Rendering|Material|SetMaterial _staticmesh_2 0 "/Game/Assets/Materials/Grid_Color_2.Grid_Color_2" :!label _label_2)
        (Rendering|Material|SetMaterial _staticmesh_2 1 "/Game/Assets/Materials/Grid_Color_1.Grid_Color_1")))
    (elif _returnvalue_4
      (goto _label_2)
      (else
        (goto _label)))))