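; Input manager that moves Character1 and Character2 together in turn-based steps and flips the map view.
; Tick merges key states and thumbsticks into a unit step per axis, X before Y, setting the GameMode's MovingATurn to block further input.
; FlipMap input negates MovePerTurn and toggles viewingtop, which also inverts Y input.
; Between moves, Tick rolls the camera by FlipSpeed until it reaches the opposite orientation.
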(event Custom|Refresh
  (bind _outactors (Actor|GetAllActorsOfClass "/Game/Blueprints/Character1.Character1_C"))
  (Variables|Default|SetCharacter1 (Utilities|Array|Get(acopy) _outactors))
  (bind _outactors_2 (Actor|GetAllActorsOfClass "/Game/Blueprints/Character2.Character2_C"))
  (Variables|Default|SetCharacter2 (Utilities|Array|Get(acopy) _outactors_2))
  (bind _outactors_3 (Actor|GetAllActorsOfClass "/Game/Blueprints/TheCamera.TheCamera_C"))
  (Variables|Default|SetTheCamera (Utilities|Array|Get(acopy) _outactors_3)))

(event EventBeginPlay
  (CallFunction|Refresh))

(event EventTick
  (params (DeltaSeconds :type Float%20%28single-precision%29))
  (bind _returnvalue (Game|GetGameMode))
  (bind _moveperturn (Variables|Default|GetMovePerTurn))
  (bind _character1 (Variables|Default|GetCharacter1))
  (bind _character2 (Variables|Default|GetCharacter2))
  (bind _ascharacter_1 (Utilities|Casting|CastToCharacter1 _character1))
  (bind _asthe_game_mode (Utilities|Casting|CastToTheGameMode _returnvalue))
  (bind _ascharacter_2 (Utilities|Casting|CastToCharacter2 _character2))
  (bind _movingaturn (Variables|/Game/Blueprints/TheGameMode.TheGameMode_C|GetMovingATurn _asthe_game_mode))
  (if (and (Utilities|IsValid (Variables|Default|GetCharacter1)) (Utilities|IsValid (Variables|Default|GetCharacter2)))
    (Utilities|FlowControl|Sequence
      (:then_0
        (if (not _movingaturn)
          (bind _x (CallFunction|GetInputX))
          (if _movingaturn
            (Default|MoveX _ascharacter_1 (Math|Conversions|ToFloat(Integer) (* _x _moveperturn)))
            (Default|MoveX _ascharacter_2 (Math|Conversions|ToFloat(Integer) (* _x _moveperturn))))))
      (:then_1
        (if (not _movingaturn)
          (bind _y (CallFunction|GetInputY))
          (if _movingaturn
            (Default|MoveY _ascharacter_1 (Math|Conversions|ToFloat(Integer) (* _y _moveperturn)))
            (Default|MoveY _ascharacter_2 (Math|Conversions|ToFloat(Integer) (* _y _moveperturn))))))
      (:then_2
        (if (not _movingaturn)
          (if (.Value (Utilities|Map|Find (Variables|Default|GetMapProperties) "animating"))
            (CallFunction|FlipMap)))))
    (else
      (CallFunction|Refresh))))

(event Input|ActionEvents|InputActionMoveLeft
  (params (Key :type Key%20Structure))
  (bind _keys (Variables|Default|GetKeys))
  (:Pressed
    (Utilities|Map|Add _keys "left" true))
  (:Released
    (Utilities|Map|Add _keys "left" false)))

(event Input|ActionEvents|InputActionMoveRight
  (params (Key :type Key%20Structure))
  (bind _keys (Variables|Default|GetKeys))
  (:Pressed
    (Utilities|Map|Add _keys "right" true))
  (:Released
    (Utilities|Map|Add _keys "right" false)))

(event Input|ActionEvents|InputActionMoveUp
  (params (Key :type Key%20Structure))
  (bind _keys (Variables|Default|GetKeys))
  (:Pressed
    (Utilities|Map|Add _keys "up" true))
  (:Released
    (Utilities|Map|Add _keys "up" false)))

(event Input|ActionEvents|InputActionMoveDown
  (params (Key :type Key%20Structure))
  (bind _keys (Variables|Default|GetKeys))
  (:Pressed
    (Utilities|Map|Add _keys "down" true))
  (:Released
    (Utilities|Map|Add _keys "down" false)))

(event Input|ActionEvents|InputActionFlipMap
  (params (Key :type Key%20Structure))
  (bind _mapproperties (Variables|Default|GetMapProperties))
  (bind _value (Utilities|Map|Find _mapproperties "viewingtop"))
  (bind _returnvalue (not _value))
  (:Pressed
    (if (not (.Value (Utilities|Map|Find _mapproperties "animating")))
      (Utilities|Map|Add _mapproperties "animating" true)
      (Utilities|Map|Add _mapproperties "viewingtop" _returnvalue)
      (if _returnvalue
        (Variables|Default|SetMovePerTurn (* (Variables|Default|GetMovePerTurn) -1))
        (else
          (Variables|Default|SetMovePerTurn (* (Variables|Default|GetMovePerTurn) -1)))))))

(fn ConstructionScript)

(fn FlipMap
  (bind _thecamera (Variables|Default|GetTheCamera))
  (bind _returnvalue (Transformation|GetActorRotation _thecamera))
  (bind _output_get (Variables|Default|SetCamera's%20Rotation (+ (Variables|Default|GetCamera's%20Rotation) (LocalVariables|GetFlipSpeed))))
  (Transformation|SetActorRotation _thecamera (Math|Rotator|MakeRotator _output_get (.pitch _returnvalue) (.yaw _returnvalue)))
  (if (.Value (Utilities|Map|Find (Variables|Default|GetMapProperties) "viewingtop"))
    (if (== (- (Math|Float|Round (+ (Variables|Default|GetCamera's%20Rotation) (LocalVariables|GetFlipSpeed))) (Math|Float|Truncate (LocalVariables|GetFlipSpeed))) 360)
      (Variables|Default|SetCamera's%20Rotation 0.0)
      (Utilities|Map|Add (Variables|Default|GetMapProperties) "animating" false :!label _label))
    (elif (== (- (Math|Float|Round (+ (Variables|Default|GetCamera's%20Rotation) (LocalVariables|GetFlipSpeed))) (Math|Float|Truncate (LocalVariables|GetFlipSpeed))) 180)
      (goto _label))))

(fn GetInputX
  (bind _keys (Variables|Default|GetKeys))
  (LocalVariables|SetAmount 0.0)
  (Utilities|FlowControl|Sequence
    (:then_0
      (if (.Value (Utilities|Map|Find _keys "right"))
        (LocalVariables|SetAmount (+ (LocalVariables|GetAmount) -1.0))))
    (:then_1
      (if (.Value (Utilities|Map|Find _keys "left"))
        (LocalVariables|SetAmount (+ (LocalVariables|GetAmount) 1.0))))
    (:then_2
      (LocalVariables|SetAmount (+ (Input|AxisValues|GetRightXThumbStick) (LocalVariables|GetAmount))))
    (:then_3
      (LocalVariables|SetAmount (+ (LocalVariables|GetAmount) (Input|AxisValues|GetLeftXThumbStick))))
    (:then_4
      (if (> (LocalVariables|GetAmount) 1.0)
        (LocalVariables|SetAmount 1.0)
        (elif (< (LocalVariables|GetAmount) -1.0)
          (bind _output_get (LocalVariables|SetAmount -1.0))))
      (if (!= 0.0 _output_get)
        (Variables|/Game/Blueprints/TheGameMode.TheGameMode_C|SetMovingATurn (.AsThe%20Game%20Mode (Utilities|Casting|CastToTheGameMode (Game|GetGameMode))) true)
        (if (> _output_get 0.0)
          (return 1)
          (else
            (return -1)))
        (else
          (return 0))))))

(fn GetInputY
  (bind _keys (Variables|Default|GetKeys))
  (LocalVariables|SetAmount 0.0)
  (Utilities|FlowControl|Sequence
    (:then_0
      (if (.Value (Utilities|Map|Find _keys "down"))
        (LocalVariables|SetAmount (+ (LocalVariables|GetAmount) -1.0))))
    (:then_1
      (if (.Value (Utilities|Map|Find _keys "up"))
        (LocalVariables|SetAmount (+ (LocalVariables|GetAmount) 1.0))))
    (:then_2
      (LocalVariables|SetAmount (+ (Input|AxisValues|GetRightYThumbStick) (LocalVariables|GetAmount))))
    (:then_3
      (LocalVariables|SetAmount (+ (LocalVariables|GetAmount) (Input|AxisValues|GetLeftYThumbStick))))
    (:then_4
      (if (> (LocalVariables|GetAmount) 1.0)
        (LocalVariables|SetAmount 1.0)
        (elif (< (LocalVariables|GetAmount) -1.0)
          (LocalVariables|SetAmount -1.0)))
      (if (.Value (Utilities|Map|Find (Variables|Default|GetMapProperties) "viewingtop"))
        _
        (else
          (bind _output_get (LocalVariables|SetAmount (* (LocalVariables|GetAmount) -1.0)))))
      (if (!= _output_get 0.0)
        (Variables|/Game/Blueprints/TheGameMode.TheGameMode_C|SetMovingATurn (.AsThe%20Game%20Mode (Utilities|Casting|CastToTheGameMode (Game|GetGameMode))) true)
        (if (> _output_get 0.0)
          (return 1)
          (else
            (return -1)))
        (else
          (return 0))))))