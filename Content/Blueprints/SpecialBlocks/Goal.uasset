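; Goal block placed on either the Top or Bottom side, reporting whether a TheCharacter is standing in it.
; Begin and end overlap toggle Pressed and write it to TheGameMode's Goals array at the index derived from Side.
; Tick re-writes true every frame while pressed.
; The construction script shifts the mesh up or down in world Z to match its Side.
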(event EventBeginPlay
  (switch Utilities|FlowControl|Switch|SwitchonSides (Variables|Default|GetSide)
    (:NewEnumerator0
      (Variables|Default|SetSideInt 0))
    (:NewEnumerator1
      (Variables|Default|SetSideInt 1))))

(event Collision|EventActorBeginOverlap
  (params (OtherActor :type Actor%20Object%20Reference))
  (Utilities|Casting|CastToTheCharacter OtherActor)
  (Variables|Default|SetPressed true)
  (Utilities|Array|SetArrayElem (Variables|/Game/Blueprints/TheGameMode.TheGameMode_C|GetGoals (.AsThe%20Game%20Mode (Utilities|Casting|CastToTheGameMode (Game|GetGameMode)))) (Variables|Default|GetSideInt) (stale Collision|EventActorEndOverlap _output_get)))

(event EventTick
  (params (DeltaSeconds :type Float%20%28single-precision%29))
  (if (Variables|Default|GetPressed)
    (Utilities|Array|SetArrayElem (Variables|/Game/Blueprints/TheGameMode.TheGameMode_C|GetGoals (.AsThe%20Game%20Mode (Utilities|Casting|CastToTheGameMode (Game|GetGameMode)))) (Variables|Default|GetSideInt) true)))

(event Collision|EventActorEndOverlap
  (params (OtherActor :type Actor%20Object%20Reference))
  (Utilities|Casting|CastToTheCharacter OtherActor)
  (bind _output_get (Variables|Default|SetPressed false))
  (Utilities|Array|SetArrayElem (Variables|/Game/Blueprints/TheGameMode.TheGameMode_C|GetGoals (.AsThe%20Game%20Mode (Utilities|Casting|CastToTheGameMode (Game|GetGameMode)))) (Variables|Default|GetSideInt) _output_get))

(fn ConstructionScript
  (bind _staticmesh (Variables|Default|GetStaticMesh))
  (bind _returnvalue (Transformation|GetWorldLocation _staticmesh))
  (switch Utilities|FlowControl|Switch|SwitchonSides (Variables|Default|GetSide)
    (:NewEnumerator0
      (Transformation|SetWorldLocationAndRotation _staticmesh (+ _returnvalue "0, 0,50.000000") "0, 0, 0" false false))
    (:NewEnumerator1
      (Transformation|SetWorldLocationAndRotation _staticmesh (- _returnvalue "0, 0,50.000000") "0, 0, 0" false false))))