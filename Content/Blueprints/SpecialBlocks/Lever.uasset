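; Lever block that toggles on or off each time the player character overlaps it, switching power for its Type.
; Plane turns orange when on and red when off.
; It writes to the game mode's Power map, re-asserting true every Tick while on (with a debug print) and setting false when switched off.
; The construction script orients and offsets Plane by Side and colors PowerPoint with the game mode's material for that Type.
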(event Collision|EventActorBeginOverlap
  (params (OtherActor :type Actor%20Object%20Reference))
  (bind _plane (Variables|Default|GetPlane))
  (Utilities|Casting|CastToTheCharacter OtherActor)
  (bind _output_get (Variables|Default|SetPressed (not (Variables|Default|GetPressed))))
  (if _output_get
    (Rendering|Material|SetMaterial _plane 0 "/Game/Assets/Materials/Orange.Orange")
    (else
      (Rendering|Material|SetMaterial _plane 0 "/Game/Assets/Materials/Red.Red")
      (Utilities|Map|Add (Variables|/Game/Blueprints/TheGameMode.TheGameMode_C|GetPower (.AsThe%20Game%20Mode (Utilities|Casting|CastToTheGameMode (Game|GetGameMode)))) (Variables|Default|GetType) false))))

(event EventTick
  (params (DeltaSeconds :type Float%20%28single-precision%29))
  (if (Variables|Default|GetPressed)
    (Development|PrintString "hry")
    (Utilities|Map|Add (Variables|/Game/Blueprints/TheGameMode.TheGameMode_C|GetPower (.AsThe%20Game%20Mode (Utilities|Casting|CastToTheGameMode (Game|GetGameMode)))) (Variables|Default|GetType) true)))

(fn ConstructionScript
  (bind _plane (Variables|Default|GetPlane))
  (switch Utilities|FlowControl|Switch|SwitchonSides (Variables|Default|GetSide)
    (:NewEnumerator0
      _)
    (:NewEnumerator1
      (Transformation|SetWorldRotation _plane "180.000000, 0, 0" false false)))
  (Transformation|SetWorldLocation _plane (+ (Transformation|GetWorldLocation _plane) "0, 0,50.099998") false false)
  (bind _asthe_game_mode (Utilities|Casting|CastToTheGameMode (Game|GetGameMode)))
  (bind _material (Default|GetMaterailfromType _asthe_game_mode (Variables|Default|GetType)))
  (Rendering|Material|SetMaterial (Variables|Default|GetPowerPoint) 0 _material))