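; PowerPad is a pressure plate block that powers its Type channel while a TheCharacter stands on it.
; Overlaps toggle Pressed and swap the Up/Down visuals and Plane height.
; While pressed, Tick rewrites true into TheGameMode's Power map every frame, and leaving writes false once.
; The construction script offsets the Box, rotates it for the Bottom side, and colors the Plane with the game mode's material for that Type.
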(event Collision|EventActorBeginOverlap
  (params (OtherActor :type Actor%20Object%20Reference))
  (Utilities|Casting|CastToTheCharacter OtherActor)
  (Variables|Default|SetPressed true)
  (CallFunction|Pushed))

(event EventTick
  (params (DeltaSeconds :type Float%20%28single-precision%29))
  (if (Variables|Default|GetPressed)
    (Utilities|Map|Add (Variables|/Game/Blueprints/TheGameMode.TheGameMode_C|GetPower (.AsThe%20Game%20Mode (Utilities|Casting|CastToTheGameMode (Game|GetGameMode)))) (Variables|Default|GetType) true)))

(event Collision|EventActorEndOverlap
  (params (OtherActor :type Actor%20Object%20Reference))
  (Utilities|Casting|CastToTheCharacter OtherActor)
  (Variables|Default|SetPressed false)
  (CallFunction|Pulled)
  (Utilities|Map|Add (Variables|/Game/Blueprints/TheGameMode.TheGameMode_C|GetPower (.AsThe%20Game%20Mode (Utilities|Casting|CastToTheGameMode (Game|GetGameMode)))) (Variables|Default|GetType) false))

(fn ConstructionScript
  (bind _box (Variables|Default|GetBox))
  (bind _returnvalue (Transformation|GetWorldLocation _box))
  (bind _returnvalue_2 (+ _returnvalue "0, 0,50.000000"))
  (switch Utilities|FlowControl|Switch|SwitchonSides (Variables|Default|GetSide)
    (:NewEnumerator0
      (Transformation|SetWorldLocationAndRotation _box _returnvalue_2 "0, 0, 0" false false))
    (:NewEnumerator1
      (Transformation|SetWorldLocationAndRotation _box _returnvalue_2 "180.000000, 0, 0" false false)))
  (bind _asthe_game_mode (Utilities|Casting|CastToTheGameMode (Game|GetGameMode)))
  (bind _material (Default|GetMaterailfromType _asthe_game_mode (Variables|Default|GetType)))
  (Rendering|Material|SetMaterial (Variables|Default|GetPlane) 0 _material))

(fn Pushed
  (Rendering|SetVisibility (Variables|Default|GetDown) true false)
  (Rendering|SetVisibility (Variables|Default|GetUp) false false)
  (Transformation|SetRelativeLocation (Variables|Default|GetPlane) "0,-1.000000,3.100000" false false))

(fn Pulled
  (Rendering|SetVisibility (Variables|Default|GetDown) false false)
  (Rendering|SetVisibility (Variables|Default|GetUp) true false)
  (Transformation|SetRelativeLocation (Variables|Default|GetPlane) "0,-1.000000,12.100000" false false))