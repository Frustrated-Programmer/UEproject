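; Stone wall block that swaps its visible meshes based on neighboring stone wall blocks.
; Construction script orients it for a Top or Bottom side.
; CheckSides line-traces four horizontal directions from an offset point, ignoring floors, gates, spawn platforms and characters, to detect a straight run along only X or Y.
; Flat shows Cube4 for a straight run, otherwise StaticMesh4 and StaticMesh5; nothing in this Blueprint calls it.
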(event Collision|EventActorBeginOverlap
  (params (OtherActor :type Actor%20Object%20Reference)))

(fn ConstructionScript
  (bind _defaultsceneroot (Variables|Default|GetDefaultSceneRoot))
  (switch Utilities|FlowControl|Switch|SwitchonSides (Variables|Default|GetSide)
    (:NewEnumerator0
      (Transformation|SetWorldRotation _defaultsceneroot "0, 0, 0" false false))
    (:NewEnumerator1
      (Transformation|SetWorldRotation _defaultsceneroot "180.000000, 0, 0" false false))))

(fn CheckSides
  (bind _defaultsceneroot (Variables|Default|GetDefaultSceneRoot))
  (bind _returnvalue (Transformation|GetWorldLocation _defaultsceneroot))
  (bind _outactors (Actor|GetAllActorsOfClass "/Game/Blueprints/FloorBox.FloorBox_C"))
  (bind _output_get (LocalVariables|SetIgnore _outactors))
  (bind _outactors_2 (Actor|GetAllActorsOfClass "/Game/Blueprints/SpecialBlocks/gate.gate_C"))
  (Utilities|Array|AppendArray _output_get _outactors_2)
  (bind _outactors_3 (Actor|GetAllActorsOfClass "/Game/Blueprints/SpecialBlocks/SpawnPlatform.SpawnPlatform_C"))
  (Utilities|Array|AppendArray _output_get _outactors_3)
  (bind _outactors_4 (Actor|GetAllActorsOfClass "/Game/Blueprints/TheCharacter.TheCharacter_C"))
  (Utilities|Array|AppendArray _output_get _outactors_4)
  (switch Utilities|FlowControl|Switch|SwitchonSides (Variables|Default|GetSide)
    (:NewEnumerator0
      (LocalVariables|SetLoc (+ _returnvalue "0, 0,75.000000")))
    (:NewEnumerator1
      (LocalVariables|SetLoc (+ _returnvalue "0, 0,-75.000000"))))
  (Utilities|FlowControl|Sequence
    (:then_0
      (bind _hit (CallFunction|CheckSide (LocalVariables|GetLoc) (+ (LocalVariables|GetLoc) "75.000000,0.000000,0.000000") (LocalVariables|GetIgnore)))
      (LocalVariables|SetX+ _hit))
    (:then_1
      (bind _hit_2 (CallFunction|CheckSide (LocalVariables|GetLoc) (+ (LocalVariables|GetLoc) "-75.000000,0.000000,0.000000") (LocalVariables|GetIgnore)))
      (LocalVariables|SetX- _hit_2))
    (:then_2
      (bind _hit_3 (CallFunction|CheckSide (LocalVariables|GetLoc) (+ (LocalVariables|GetLoc) "0.000000,75.000000,0.000000") (LocalVariables|GetIgnore)))
      (LocalVariables|SetY+ _hit_3))
    (:then_3
      (bind _hit_4 (CallFunction|CheckSide (LocalVariables|GetLoc) (+ (LocalVariables|GetLoc) "0.000000,-75.000000,0.000000") (LocalVariables|GetIgnore)))
      (LocalVariables|SetY- _hit_4))
    (:then_4
      (if (Math|Boolean|ORBoolean (LocalVariables|GetX+) (LocalVariables|GetX-) (LocalVariables|GetY+) (LocalVariables|GetY-))
        (if (Math|Boolean|ANDBoolean (LocalVariables|GetX+) (LocalVariables|GetX-) (not (or (LocalVariables|GetY+) (LocalVariables|GetY-))))
          ;[1 1 1] X+ & X- = true, Y+ & Y- = false
          (return true)
          (elif (Math|Boolean|ANDBoolean (not (or (LocalVariables|GetX+) (LocalVariables|GetX-))) (LocalVariables|GetY+) (LocalVariables|GetY-))
            ;[1 1 1] X+ & X- = false, Y+ & Y- = true
            (return true)
            (else
              (return false))))
        (else
          (return false))))))

(fn CheckSide
  (params (Start :type Vector) (End :type Vector) (Ignore :type Array%20of%20Actor%20Object%20References))
  (bind (_outhit _returnvalue) (Collision|LineTraceByChannel Start End "TraceTypeQuery1" false Ignore "None" true "(R=0.166315,G=0.083596,B=1.000000,A=1.000000)"))
  (Utilities|Casting|CastToStone_wall_Block (.hitactor _outhit)
    (:then
      (return _returnvalue))
    (:CastFailed
      (return false))))

(fn Flat
  (bind _cube4 (Variables|Default|GetCube4))
  (bind _staticmesh4 (Variables|Default|GetStaticMesh4))
  (bind _staticmesh5 (Variables|Default|GetStaticMesh5))
  (bind _flat (CallFunction|CheckSides))
  (if _flat
    (Rendering|SetVisibility _cube4 true false)
    (Rendering|SetVisibility _staticmesh4 false false)
    (Rendering|SetVisibility _staticmesh5 false false)
    (else
      (Rendering|SetVisibility _cube4 false false)
      (Rendering|SetVisibility _staticmesh4 true false)
      (Rendering|SetVisibility _staticmesh5 true false))))