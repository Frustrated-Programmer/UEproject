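; Timed button block that powers its Type channel in TheGameMode's Power map once TheCharacter overlaps it.
; Overlap lowers the button and loads Timer from Length; Tick reasserts power, rotates the clock arrow from Timer, and releases both at zero.
; Nothing in these graphs decrements Timer.
; Construction orients the block by Side, offsets it vertically and colors the power line with the game mode's material for Type.
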(event Collision|EventActorBeginOverlap
  (params (OtherActor :type Actor%20Object%20Reference))
  (Utilities|Casting|CastToTheCharacter OtherActor)
  (Variables|Default|SetPressed true)
  (Variables|Default|SetTimer (Variables|Default|GetLength))
  (Components|StaticMesh|SetStaticMesh (Variables|Default|GetStaticMesh) "/Game/Assets/Models/Timer_button_down.Timer_button_down")
  (Transformation|SetRelativeLocation (Variables|Default|GetClock) "0, 0,15.200000" false false))

(event EventTick
  (params (DeltaSeconds :type Float%20%28single-precision%29))
  (bind _returnvalue (Game|GetGameMode))
  (bind _asthe_game_mode (Utilities|Casting|CastToTheGameMode _returnvalue))
  (bind _power (Variables|/Game/Blueprints/TheGameMode.TheGameMode_C|GetPower _asthe_game_mode))
  (if (Variables|Default|GetPressed)
    (Utilities|Map|Add _power (Variables|Default|GetType) true)
    (if (== (Variables|Default|GetTimer) 0)
      (Utilities|Map|Add _power (Variables|Default|GetType) false)
      (Variables|Default|SetPressed false)
      (Components|StaticMesh|SetStaticMesh (Variables|Default|GetStaticMesh) "/Game/Assets/Models/Timer_button_up.Timer_button_up")
      (Transformation|SetRelativeLocation (Variables|Default|GetClock) "0, 0,18.778534" false false))
    (Transformation|SetRelativeRotation (Variables|Default|GetArrow) (Math|Rotator|MakeRotator 0.0 0.0 (* (Variables|Default|GetTimer) 3e+01)) false false)))

(fn ConstructionScript
  (bind _defaultsceneroot (Variables|Default|GetDefaultSceneRoot))
  (switch Utilities|FlowControl|Switch|SwitchonSides (Variables|Default|GetSide)
    (:NewEnumerator0
      _)
    (:NewEnumerator1
      (Transformation|SetWorldRotation _defaultsceneroot "180.000000,180.000000, 0" false false)))
  (Transformation|SetWorldLocation _defaultsceneroot (+ (Transformation|GetWorldLocation _defaultsceneroot) "0, 0,50.099998") false false)
  (bind _asthe_game_mode (Utilities|Casting|CastToTheGameMode (Game|GetGameMode)))
  (bind _material (Default|GetMaterailfromType _asthe_game_mode (Variables|Default|GetType)))
  (Rendering|Material|SetMaterial (Variables|Default|GetPowerLine) 0 _material))