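; TheCharacter is one of two player characters that move in discrete steps along X or Y, with particle templates chosen by the PlayerOne flag.
; MoveX and MoveY start a step only if a line trace to the target is clear and a vertical trace there hits something, then set Facing.
; Tick advances the root by the GameMode's OverallSpeed until Step reaches its limit.
; DoneMoving then clears movement state and that player's GameMode moving flag.
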(event EventTick
  (params (DeltaSeconds :type Float%20%28single-precision%29))
  (bind _returnvalue (Game|GetGameMode))
  (bind _defaultsceneroot1 (Variables|Default|GetDefaultSceneRoot1))
  (bind _returnvalue_2 (Transformation|GetWorldLocation _defaultsceneroot1))
  (bind _asthe_game_mode (Utilities|Casting|CastToTheGameMode _returnvalue))
  (bind _overallspeed (Variables|/Game/Blueprints/TheGameMode.TheGameMode_C|GetOverallSpeed _asthe_game_mode))
  (if (Variables|Default|GetMoving)
    (Transformation|SetWorldLocation (Variables|Default|GetDefaultSceneRoot1) (Math|Vector|MakeVector (+ (* _overallspeed (Variables|Default|GetX)) (.x _returnvalue_2)) (+ (* _overallspeed (Variables|Default|GetY)) (.y _returnvalue_2)) (.z _returnvalue_2)) false false)
    (bind _output_get (Variables|Default|SetStep (+ _overallspeed (Variables|Default|GetStep))))
    (if (>= _output_get 1e+02)
      (CallFunction|DoneMoving))))

(fn ConstructionScript
  (bind _particlesystem (Variables|Default|GetParticleSystem))
  (bind _particlesystem1 (Variables|Default|GetParticleSystem1))
  (if (Variables|Default|GetPlayerOne?)
    (Effects|Components|ParticleSystem|SetTemplate _particlesystem "/Game/Assets/Particles/B_ParticleMaker.B_ParticleMaker")
    (Effects|Components|ParticleSystem|SetTemplate _particlesystem1 "/Game/Assets/Particles/B_ParticleMaker.B_ParticleMaker")
    (else
      (Effects|Components|ParticleSystem|SetTemplate _particlesystem "/Game/Assets/Particles/W_ParticleMaker.W_ParticleMaker")
      (Effects|Components|ParticleSystem|SetTemplate _particlesystem1 "/Game/Assets/Particles/W_ParticleMaker.W_ParticleMaker"))))

(fn MoveX
  (params (X :type Float%20%28single-precision%29) (Ignore :type Array%20of%20Actor%20Object%20References) (Positive :type Boolean))
  (bind _returnvalue (Game|GetGameMode))
  (bind _defaultsceneroot1 (Variables|Default|GetDefaultSceneRoot1))
  (bind _returnvalue_2 (Transformation|GetWorldLocation _defaultsceneroot1))
  (bind _asthe_game_mode (Utilities|Casting|CastToTheGameMode _returnvalue))
  (bind (_x _y _z) (Math|Vector|BreakVector _returnvalue_2))
  (bind _returnvalue_3 (+ X _x))
  (bind _returnvalue_4 (Math|Vector|MakeVector _returnvalue_3 _y _z))
  (bind (_x_2 _y_2) (Math|Vector|BreakVector _returnvalue_4))
  (if (not (Variables|Default|GetMoving))
    (if (!= X 0.0)
      (bind _returnvalue_5 (Collision|LineTraceByChannel _returnvalue_2 _returnvalue_4 "TraceTypeQuery1" false Ignore "None"))
      (if (not _returnvalue_5)
        (bind _returnvalue_6 (Collision|LineTraceByChannel _returnvalue_4 (Math|Vector|MakeVector _x_2 _y_2 5e+02) "TraceTypeQuery1" false Ignore "None"))
        (if _returnvalue_6
          (if (Variables|Default|GetPlayerOne?)
            (Variables|/Game/Blueprints/TheGameMode.TheGameMode_C|SetChar1Moving _asthe_game_mode true)
            (else
              (Variables|/Game/Blueprints/TheGameMode.TheGameMode_C|SetChar2Moving _asthe_game_mode true)))
          (Variables|Default|SetMoving true)
          (Variables|Default|SetX (/ X 1e+02))
          (if Positive
            (Variables|Default|SetFacing "NewEnumerator0")
            (else
              (Variables|Default|SetFacing "NewEnumerator1"))))))))

(fn MoveY
  (params (Y :type Float%20%28single-precision%29) (Ignore :type Array%20of%20Actor%20Object%20References) (Positive :type Boolean))
  (bind _returnvalue (Game|GetGameMode))
  (bind _defaultsceneroot1 (Variables|Default|GetDefaultSceneRoot1))
  (bind _returnvalue_2 (Transformation|GetWorldLocation _defaultsceneroot1))
  (bind _asthe_game_mode (Utilities|Casting|CastToTheGameMode _returnvalue))
  (bind (_x _y _z) (Math|Vector|BreakVector _returnvalue_2))
  (bind _returnvalue_3 (+ Y _y))
  (bind _returnvalue_4 (Math|Vector|MakeVector _x _returnvalue_3 _z))
  (bind (_x_2 _y_2) (Math|Vector|BreakVector _returnvalue_4))
  (if (not (Variables|Default|GetMoving))
    (if (!= Y 0.0)
      (bind _returnvalue_5 (Collision|LineTraceByChannel _returnvalue_2 _returnvalue_4 "TraceTypeQuery1" false Ignore "None" true "(R=1.000000,G=0.000000,B=0.834424,A=1.000000)" "(R=0.000000,G=0.259094,B=1.000000,A=1.000000)"))
      (if (not _returnvalue_5)
        (bind _returnvalue_6 (Collision|LineTraceByChannel _returnvalue_4 (Math|Vector|MakeVector _x_2 _y_2 5e+02) "TraceTypeQuery1" false Ignore "None" true "(R=0.000000,G=1.000000,B=0.075142,A=1.000000)" "(R=1.000000,G=0.191836,B=0.000000,A=1.000000)"))
        (if _returnvalue_6
          (if (Variables|Default|GetPlayerOne?)
            (Variables|/Game/Blueprints/TheGameMode.TheGameMode_C|SetChar1Moving _asthe_game_mode true)
            (else
              (Variables|/Game/Blueprints/TheGameMode.TheGameMode_C|SetChar2Moving _asthe_game_mode true)))
          (Variables|Default|SetMoving true)
          (Variables|Default|SetY (/ Y 1e+02))
          (if Positive
            (Variables|Default|SetFacing "NewEnumerator2")
            (else
              (Variables|Default|SetFacing "NewEnumerator3"))))))))

(fn DoneMoving
  (bind _asthe_game_mode (Utilities|Casting|CastToTheGameMode (Game|GetGameMode))
    (:then
      (if (Variables|Default|GetPlayerOne?)
        (Variables|/Game/Blueprints/TheGameMode.TheGameMode_C|SetChar1Moving _asthe_game_mode false)
        (else
          (Variables|/Game/Blueprints/TheGameMode.TheGameMode_C|SetChar2Moving _asthe_game_mode false)))
      (Variables|Default|SetMoving false)
      (Variables|Default|SetX 0.0)
      (Variables|Default|SetY 0.0)
      (Variables|Default|SetStep 0.0))
    (:CastFailed
      (Development|PrintString "What happened? Char1 couldn't cast to TheGameMode when DoneMoving" true true "(R=1.000000,G=0.046953,B=0.000000,A=1.000000)" 2e+01))))