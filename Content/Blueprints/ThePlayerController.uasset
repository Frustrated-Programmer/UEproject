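; Player controller that handles the move from the intro screen to the main menu and the in-level overlay.
; BeginPlay shows the Intro widget and the mouse cursor.
; While the Intro flag is set, a keyboard key or Any Key press swaps all widgets for MainMenu and clears the flag.
; StartLevel adds the GameOverlay widget to the player screen, leaving its Level input unused.
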(event EventBeginPlay
  (bind _self self)
  (bind _returnvalue (UserInterface|CreateWidget "/Game/Assets/GUI/Intro.Intro_C" _self))
  (UserInterface|Viewport|AddtoPlayerScreen _returnvalue)
  (Variables|/Script/Engine.PlayerController|SetbShowMouseCursor _self true))

(event EventTick
  (params (DeltaSeconds :type Float%20%28single-precision%29)))

(event Input|ActionEvents|InputActionAnyKey
  (params (Key :type Key%20Structure))
  (:Pressed
    (if (Variables|Default|GetIntro)
      (Viewport|RemoveAllWidgets)
      (bind _returnvalue (UserInterface|CreateWidget "/Game/Assets/GUI/MainMenu.MainMenu_C" self))
      (UserInterface|Viewport|AddtoViewport _returnvalue 0)
      (Variables|Default|SetIntro false))))

(event Input|ActionEvents|InputActionAny
  (params (Key :type Key%20Structure))
  (:Pressed
    (if (Class|KismetInputLibrary|KeyIsKeyboardKey Key)
      (if (Variables|Default|GetIntro)
        (Viewport|RemoveAllWidgets)
        (bind _returnvalue (UserInterface|CreateWidget "/Game/Assets/GUI/MainMenu.MainMenu_C" self))
        (UserInterface|Viewport|AddtoViewport _returnvalue 0)
        (Variables|Default|SetIntro false)))))

(fn ConstructionScript)

(fn StartLevel
  (params (Level :type Integer))
  (bind _returnvalue (UserInterface|CreateWidget "/Game/Assets/GUI/GameOverlay.GameOverlay_C" self))
  (UserInterface|Viewport|AddtoPlayerScreen _returnvalue))